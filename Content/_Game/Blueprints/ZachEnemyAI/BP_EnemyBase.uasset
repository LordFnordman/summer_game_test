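; Base enemy character that chases the first-person player and damages them on contact.
; A looping AIMoveTo re-targets the player after a pause, whether the move succeeds or fails.
; DamageZone overlaps send damage through BPI_Damageable, gated by a DoOnce that resets after a cooldown or any end overlap.
; JumpCollision overlaps trigger jumps, and the construction script applies configurable speed, capsule scale and jump velocity.
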(event `Go After Player`
  (bind _returnvalue (`GameplayStatics.GetActorOfClass` "/Game/_Game/Blueprints/BP_FirstPersonCharacter.BP_FirstPersonCharacter_C" :!label _label))
  (`|AIMoveTo` self (0.0 0.0 0.0) _returnvalue
    (:`OnSuccess`
      (`KismetSystemLibrary.PrintString` "INFO: AI Reach Player Success. Continuing after Player"))
    (:`OnFail`
      (`KismetSystemLibrary.PrintString` "INFO: AI Reach Player Failiure. Retrying...")))
  (`KismetSystemLibrary.Delay` (`self.Movement Pause Duration`))
  (`self.Go After Player`))

(event `self.ReceiveBeginPlay`
  (bind _asbp_first_person_character (cast `/Game/_Game/Blueprints/BP_FirstPersonCharacter` (`GameplayStatics.GetPlayerCharacter` 0)))
  (set `self.Player` _asbp_first_person_character)
  (goto _label))

(event `self.Damage Zone.OnComponentBeginOverlap`
  (params (OverlappedComponent :type "PrimitiveComponent Object Reference") (OtherActor :type "Actor Object Reference") (OtherComp :type "PrimitiveComponent Object Reference") (OtherBodyIndex :type Integer) (bFromSweep :type Boolean) (SweepResult :type "HitResult Structure (by ref)"))
  (if (`self.ActorHasTag` OtherActor "Player")
    (if (`KismetSystemLibrary.DoesImplementInterface` OtherActor "/Game/_Game/Blueprints/Interfaces/BPI_Damageable.BPI_Damageable_C")
      (`/Engine/EditorBlueprintResources/StandardMacros.DoOnce` false :!label _label_2
        (:`Completed`
          (message `/Game/_Game/Blueprints/Interfaces/BPI_Damageable.TakeDamage` OtherActor (`self.Enemy Damage`) "NewEnumerator0")
          (`KismetSystemLibrary.PrintString` "Enemy has Damaged Player!" true true (struct :`R` 1.0 :`A` 1.0) 4.0)
          (`KismetSystemLibrary.Delay` (`self.Atack Cooldown`))
          (goto _label_2 :!via `Reset`))))))

(event `self.Damage Zone.OnComponentEndOverlap`
  (params (OverlappedComponent :type "PrimitiveComponent Object Reference") (OtherActor :type "Actor Object Reference") (OtherComp :type "PrimitiveComponent Object Reference") (OtherBodyIndex :type Integer))
  (goto _label_2 :!via `Reset`))

(event `self.Jump Collision.OnComponentBeginOverlap`
  (params (OverlappedComponent :type "PrimitiveComponent Object Reference") (OtherActor :type "Actor Object Reference") (OtherComp :type "PrimitiveComponent Object Reference") (OtherBodyIndex :type Integer) (bFromSweep :type Boolean) (SweepResult :type "HitResult Structure (by ref)"))
  (`self.Jump`))

(fn `UserConstructionScript`
  (bind _charactermovement (`self.CharacterMovement`))
  (set `CharacterMovementComponent.MaxWalkSpeed` (`self.Enemy Speed`) _charactermovement)
  (`SceneComponent.SetWorldScale3D` (`self.CapsuleComponent`) (`self.Enemy Scale`))
  (set `CharacterMovementComponent.JumpZVelocity` (`self.Jump Z Velocity`) _charactermovement))