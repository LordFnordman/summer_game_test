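; BP_ProceduralSpawningManager runs endless enemy waves, tracking round, enemies left and score.
; On BeginPlay it gathers Note actors as spawn points, then each round spawns random enemy types at random points.
; EnemyKilled adds score and, once none remain, raises the spawn count by a multiplier and starts the next round after delays.
; A test-only K key destroys all BP_EnemyBase actors, counting each as a kill.
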(event `Key|K`
  (params (Key :type "Key Structure"))
  ;[1 0.7333 0] Testing - Do Not Include in Public or Showcase Releases
  (:`Pressed`
    (`/Engine/EditorBlueprintResources/StandardMacros.DoOnce` false :!label _label
      (:`Completed`
        (bind _outactors (`GameplayStatics.GetAllActorsOfClass` "/Game/_Game/Blueprints/ZachEnemyAI/BP_EnemyBase.BP_EnemyBase_C"))
        (for _array_element _outactors
          (`self.K2_DestroyActor` _array_element)
          (`self.Enemy Killed`))
        (goto _label :!via `Reset`)))))

(event `self.ReceiveBeginPlay`
  ;[0.5406 1 0.5633] Game Set Up
  (`|ExecutionSequence`
    (:`then_0`
      (`KismetSystemLibrary.Delay` 3.0)
      (bind _outactors (`GameplayStatics.GetAllActorsOfClass` "/Script/Engine.Note"))
      (set `self.Enemy Spawn Points` _outactors)
      (`KismetSystemLibrary.PrintString` "INFO: Enemy Spawning System Initiated" true true (struct :`R` 1.0 :`G` 0.026156 :`A` 1.0) 4.0)
      (`KismetSystemLibrary.Delay` 2.0)
      (`KismetSystemLibrary.PrintString` (`KismetStringLibrary.Concat_StrStr` "INFO: " (`KismetStringLibrary.Conv_IntToString` (`KismetArrayLibrary.Array_Length` _outactors)) " enemy spawn points found! Starting Procedural Spawn Waves") true true (struct :`R` 1.0 :`B` 0.01308 :`A` 1.0) 5.0)
      (`KismetSystemLibrary.Delay` 3.0)
      (`self.Spawn a New Round`))
    (:`then_1`
      ;[1 0.7333 0] Testing
      (`self.EnableInput` (`GameplayStatics.GetPlayerController` 0)))))

(event `Increase Difficulty`
  ;[0.1922 0.2118 0.4157] Difficulty Incrementer
  (bind _output_get (set `self.Amount of Enemies to Spawn` (* (`self.Amount of Enemies to Spawn`) 1.2)))
  (`KismetSystemLibrary.PrintString` (`KismetStringLibrary.Concat_StrStr` "INFO: Difficulty Increased to " (`KismetStringLibrary.Conv_IntToString` (`KismetMathLibrary.FTrunc` _output_get)) " enemies per round") true true (struct :`R` 1.0 :`B` 0.010851 :`A` 1.0) 5.0))

(event `Spawn a New Round`
  ;[0.1922 0.2118 0.4157] Enemy Spawner/New Round Starter
  (bind _result (`/Engine/EditorBlueprintResources/StandardMacros.IncrementInt` (`self.Round`))
    (:`  `
      (`KismetSystemLibrary.PrintString` (`KismetStringLibrary.Concat_StrStr` "INFO: Starting Round " (`KismetStringLibrary.Conv_IntToString` _result)) true true (struct :`R` 1.0 :`B` 0.777538 :`A` 1.0) 5.0)
      (for _ (range 1 (+ (`KismetMathLibrary.FTrunc` (`self.Amount of Enemies to Spawn`)) 1))
        (`/Engine/EditorBlueprintResources/StandardMacros.IncrementInt` (`self.Enemies Left`)
          (:`  `
            (bind _returnvalue (`AIBlueprintHelperLibrary.SpawnAIFromClass` (`KismetArrayLibrary.Array_Random` (`self.Enemy Type Array`)) null (`self.K2_GetActorLocation` (`KismetArrayLibrary.Array_Random` (`self.Enemy Spawn Points`))) (struct) false null))
            (`KismetSystemLibrary.PrintString` (`KismetStringLibrary.Concat_StrStr` (`KismetSystemLibrary.GetClassDisplayName` (`GameplayStatics.GetObjectClass` _returnvalue)) "Spawned") true true (struct :`G` 0.08557 :`B` 1.0 :`A` 1.0) 4.0))))
      (`KismetSystemLibrary.PrintString` "INFO: Spawning Complete" true true (struct :`R` 1.0 :`B` 0.775802 :`A` 1.0) 5.0))))

(event `Enemy Killed`
  ;[1 0.0625 0.0625] Enemy Killed Protocol
  (`KismetSystemLibrary.PrintString` " INFO: Enemy Killed" true true (struct :`R` 0.088547 :`G` 1.0 :`A` 1.0) 3.0)
  (bind _result (`/Engine/EditorBlueprintResources/StandardMacros.DecrementInt` (`self.Enemies Left`))
    (:`  `
      (if (<= _result 0)
        (`|ExecutionSequence`
          (:`then_0`
            (bind _result_2 (`/Engine/EditorBlueprintResources/StandardMacros.IncrementInt` (`self.Score`) :!label _label_2)
              (:`  `
                (`KismetSystemLibrary.PrintString` (`KismetStringLibrary.Concat_StrStr` "Score: " (`KismetStringLibrary.Conv_IntToString` _result_2))))))
          (:`then_1`
            (`KismetSystemLibrary.PrintString` "INFO: Final Enemy Killed. Round Ending..." true true (struct :`R` 1.0 :`B` 0.699787 :`A` 1.0) 5.0)
            (`KismetSystemLibrary.Delay` 4.0)
            (`self.Increase Difficulty`)
            (`KismetSystemLibrary.Delay` 5.0)
            (`self.Spawn a New Round`)))
        (else
          (goto _label_2))))))

(fn `UserConstructionScript`)