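; A placeable powerup pickup actor whose selected type sets its mesh in the editor and the value it grants when picked up.
; The construction script applies the mesh from GetPowerupDetails for the selected type.
; When an actor implementing BPI_TakePowerup overlaps the mesh with a capsule component, it receives a PowerupMessage with type and value, then the pickup destroys itself.
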(event `self.PowerupMesh.OnComponentBeginOverlap`
  (params (OverlappedComponent :type "PrimitiveComponent Object Reference") (OtherActor :type "Actor Object Reference") (OtherComp :type "PrimitiveComponent Object Reference") (OtherBodyIndex :type Integer) (bFromSweep :type Boolean) (SweepResult :type "HitResult Structure (by ref)"))
  ;[1 1 1] Make sure only the correct thing triggers the powerup
  (if (`KismetSystemLibrary.DoesImplementInterface` OtherActor "/Game/_Game/Blueprints/Interfaces/BPI_TakePowerup.BPI_TakePowerup_C")
    (cast `CapsuleComponent` OtherComp)
    ;[1 1 1] Calls powerup function and destroys the powerup
    (message `/Game/_Game/Blueprints/Interfaces/BPI_TakePowerup.Powerup` OtherActor (`self.PowerUpSelected`) (`.Value_8_BECAFC6D48F78A4F7A94D5877BC8180F` (break `/Game/_Game/Blueprints/Structs/PowerupInfo` (`self.GetPowerupDetails`))))
    (`self.K2_DestroyActor`)))

(fn `UserConstructionScript`
  (bind (_powerupdetails _returnvalue) (`self.GetPowerupDetails`))
  ;[1 1 1] Allows for changing of powerup type in the editor
  (`KismetSystemLibrary.LogString` "Tried Selecting a powerup which doesnt exist" _returnvalue)
  (`StaticMeshComponent.SetStaticMesh` (`self.PowerupMesh`) (`.Mesh_5_E3E9C0ED4CF9DFA9B57FC59FBC74FE6C` (break `/Game/_Game/Blueprints/Structs/PowerupInfo` _powerupdetails))))