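; BP_Ball is a bouncing projectile ball that damages and knocks back what it hits, and can itself be knocked or redirected.
; ProjectileMovement sets normal gravity after a NoGravity delay, while knockback events overwrite its velocity or change only its direction.
; Sphere hits send truncated speed-scaled damage and fixed-force knockback through interfaces, then ChangeSpeed damps velocity, harder at high speed and to zero when slow.
; Debug prints show velocity and damage.
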(event `self.ReceiveBeginPlay`
  ;[1 1 1] Reenables Gravity after some time
  (`KismetSystemLibrary.Delay` (`self.NoGravity`))
  (set `ProjectileMovementComponent.ProjectileGravityScale` 1.0 (`self.ProjectileMovement`)))

(event `/Game/_Game/Blueprints/Interfaces/BPI_Knockback.ChangeKnockbackDirection`
  (params (NewDirection :type "Vector Structure"))
  ;[1 1 1] Changes direction projectile is moving
  (set `MovementComponent.Velocity` (* (`KismetMathLibrary.Normal` NewDirection) (`KismetMathLibrary.VSize` (`MovementComponent.Velocity` (`self.ProjectileMovement`)))) (`self.ProjectileMovement`)))

(event `/Game/_Game/Blueprints/Interfaces/BPI_Knockback.TakeKnockback`
  (params (Force :type "Float (double-precision)") (Direction :type "Vector Structure"))
  (bind _output_get (set `MovementComponent.Velocity` (* (`/Game/_Game/Blueprints/FunctionLibraries/BFL_Combat.CalculateKnockback` 1.0 Force) Direction 0.1) (`self.ProjectileMovement`)))
  (`KismetSystemLibrary.PrintString` (`KismetStringLibrary.Conv_VectorToString` _output_get) true true (struct :`G` 0.66 :`B` 1.0 :`A` 1.0) 2.0 "Vel2"))

(event `self.ProjectileMovement.OnProjectileBounce`
  (params (ImpactResult :type "HitResult Structure (by ref)") (ImpactVelocity :type "Vector Structure (by ref)")))

(event `self.Sphere.OnComponentHit`
  (params (HitComponent :type "PrimitiveComponent Object Reference") (OtherActor :type "Actor Object Reference") (OtherComp :type "PrimitiveComponent Object Reference") (NormalImpulse :type "Vector Structure") (Hit :type "HitResult Structure (by ref)"))
  (bind _projectilemovement (`self.ProjectileMovement`))
  (bind _damageoutput (`/Game/_Game/Blueprints/FunctionLibraries/BFL_Combat.SpeedToDamage` (`self.BaseDamage`) (`KismetMathLibrary.VSize` (`MovementComponent.Velocity` (`self.ProjectileMovement`)))))
  (`|ExecutionSequence`
    (:`then_0`
      ;[1 1 1] Potentially swap to an overlap to prevent unneccessary bouncing?
      (if (`KismetSystemLibrary.DoesImplementInterface` OtherActor "/Game/_Game/Blueprints/Interfaces/BPI_Damageable.BPI_Damageable_C")
        (message `/Game/_Game/Blueprints/Interfaces/BPI_Damageable.TakeDamage` OtherActor (`KismetMathLibrary.Conv_IntToDouble` (`KismetMathLibrary.FTrunc` _damageoutput)) "NewEnumerator0")
        (`KismetSystemLibrary.PrintString` (`KismetStringLibrary.BuildString_Double` "Damage Dealt:" "" _damageoutput))
        ;[1 1 1] Deals knockback to things touching the ball
        (if (`KismetSystemLibrary.DoesImplementInterface` OtherActor "/Game/_Game/Blueprints/Interfaces/BPI_Knockback.BPI_Knockback_C")
          (message `/Game/_Game/Blueprints/Interfaces/BPI_Knockback.TakeKnockback` OtherActor 100.0 (`/Game/_Game/Blueprints/FunctionLibraries/BFL_Combat.KnockbackDirection` (`self.K2_GetActorLocation`) (`self.K2_GetActorLocation` OtherActor))))))
    (:`then_1`
      ;[1 1 1] Changes ball speed on a bounce
      (set `MovementComponent.Velocity` (* (`KismetMathLibrary.Normal` (`MovementComponent.Velocity` _projectilemovement)) (`self.ChangeSpeed` (`KismetMathLibrary.VSize` (`MovementComponent.Velocity` (`self.ProjectileMovement`))))) _projectilemovement))))

(event `self.ReceiveTick`
  (params (DeltaSeconds :type "Float (single-precision)"))
  ;[1 1 1] Debug
  (`KismetSystemLibrary.PrintString` (`KismetStringLibrary.Conv_DoubleToString` (`KismetMathLibrary.VSize` (`MovementComponent.Velocity` (`self.ProjectileMovement`)))) true true (struct :`G` 0.66 :`B` 1.0 :`A` 1.0) 2.0 "Velocity"))

(fn `CalculateDamage`
  (returns (DamageAmount :type "Float (double-precision)"))
  (return 10.0))

(fn `ChangeSpeed`
  (params (CurrentSpeed :type "Float (double-precision)"))
  (returns (NewSpeed :type "Float (double-precision)"))
  ;[1 1 1] Determines how much to change speed by
  (`/Engine/EditorBlueprintResources/StandardMacros.CompareFloat` CurrentSpeed 2500.0
    (:`>`
      (return (* (`local.CurrentSpeed`) 0.93)))
    (:`==`
      _)
    (:`<`
      _))
  (`/Engine/EditorBlueprintResources/StandardMacros.CompareFloat` (`local.CurrentSpeed`) 100.0
    (:`>`
      (return (* (`local.CurrentSpeed`) 0.97)))
    (:`==`
      _)
    (:`<`
      _))
  (return 0.0))

(fn `UserConstructionScript`)