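; Environment function library whose BounceWall function determines which way an object, noted as the ball, bounces off a wall trigger.
; A dot product of the trigger's forward vector and the direction to the object picks the side.
; In front, it passes trigger location and location plus forward to KnockbackDirection; behind, it negates that whole endpoint sum.
; An exactly zero dot product has no handled branch.
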(fn `Bounce Wall`
  (params (Trigger :type "BoxComponent Object Reference") (AffectedObject :type "Actor Object Reference"))
  (returns (NewDirection :type "Vector Structure"))
  (locals (BounceLocation :type "Vector Structure") (BounceDirection :type "Vector Structure"))
  (bind _returnvalue (`SceneComponent.K2_GetComponentLocation` Trigger))
  (bind _returnvalue_2 (`SceneComponent.GetForwardVector` Trigger))
  (bind _bouncelocation (`local.BounceLocation`))
  (bind _bouncelocation_2 (`local.BounceLocation`))
  ;[1 1 1] Determines which way the ball should bounce
  (set `local.BounceLocation` _returnvalue)
  (set `local.BounceDirection` _returnvalue_2)
  (`/Engine/EditorBlueprintResources/StandardMacros.CompareFloat` (`KismetMathLibrary.Dot_VectorVector` (`KismetMathLibrary.Normal` (- (`Actor.K2_GetActorLocation` AffectedObject) _returnvalue)) _returnvalue_2)
    (:`>`
      ;[1 1 1] Applies Knockback
      (return (`/Game/_Game/Blueprints/FunctionLibraries/BFL_Combat.KnockbackDirection` _bouncelocation_2 (+ (`local.BounceDirection`) _bouncelocation_2))))
    (:`<`
      (return (`/Game/_Game/Blueprints/FunctionLibraries/BFL_Combat.KnockbackDirection` _bouncelocation (* (+ _bouncelocation (`local.BounceDirection`)) -1.0))))))