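; BFL_Combat is a Blueprint function library of combat math for damage and knockback.
; CalculateDamage scales damage by a percentage resistance and returns it negated, as a signed change.
; SpeedToDamage scales damage by the square root of speed relative to DefaultSpeed.
; Knockback direction is the normalized vector between hit origin and end, while CalculateKnockback currently returns the force unchanged, ignoring Weight.
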(fn `CalculateDamage`
  (params (Damage :type "Float (double-precision)") (DamageResistance :type "Float (double-precision)"))
  (returns (NewDamage :type "Float (double-precision)"))
  (return (* Damage (`self.CalculateDamageResistance` DamageResistance) -1.0)))

(fn `CalculateDamageResistance`
  (params (ResistAmount :type "Float (double-precision)"))
  (returns (DamageResistance :type "Float (double-precision)"))
  (return (- 1.0 (/ ResistAmount 100.0))))

(fn `CalculateKnockback`
  (params (Weight :type "Float (double-precision)") (KnockbackForce :type "Float (double-precision)"))
  (returns (NewKnockbackForce :type "Float (double-precision)"))
  (return KnockbackForce))

(fn `KnockbackDirection`
  (params (HitOrigin :type "Vector Structure") (HitEnd :type "Vector Structure"))
  (returns (Direction :type "Vector Structure"))
  (return (`KismetMathLibrary.Normal` (- HitEnd HitOrigin))))

(fn `SpeedToDamage`
  (params (DamageInput :type "Float (double-precision)") (Speed :type "Float (double-precision)"))
  (returns (DamageOutput :type "Float (double-precision)"))
  (locals (DefaultSpeed :type "Float (double-precision)" :default 2500.0))
  (return (* DamageInput (`KismetMathLibrary.Sqrt` (/ Speed (`local.DefaultSpeed`))))))